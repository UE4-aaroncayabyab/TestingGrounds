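; Shipping-container style terrain prop with a body mesh and left and right doors, given a random color.
; The construction script derives ContainerColor from a random unit vector, so it re-rolls whenever construction reruns and can contain negative channels.
; It creates dynamic material instances on slot 0 of all three meshes and sets their "diffuse color" parameter to that shared color.
; The event graph has no active logic.
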(fn `UserConstructionScript`
  (bind _containerdoorr (`self.ContainerDoorR`))
  (bind _staticmeshcomponent (`self.StaticMeshComponent`))
  (bind _containerdoorl (`self.ContainerDoorL`))
  (set `self.ContainerColor` (`KismetMathLibrary.Conv_VectorToLinearColor` (`KismetMathLibrary.RandomUnitVector`)))
  (bind _returnvalue (`PrimitiveComponent.CreateDynamicMaterialInstance` _staticmeshcomponent 0 (`PrimitiveComponent.GetMaterial` _staticmeshcomponent 0)))
  (`MaterialInstanceDynamic.SetVectorParameterValue` _returnvalue "diffuse color" (`self.ContainerColor`))
  (bind _returnvalue_2 (`PrimitiveComponent.CreateDynamicMaterialInstance` _containerdoorl 0 (`PrimitiveComponent.GetMaterial` _containerdoorl 0)))
  (`MaterialInstanceDynamic.SetVectorParameterValue` _returnvalue_2 "diffuse color" (`self.ContainerColor`))
  (bind _returnvalue_3 (`PrimitiveComponent.CreateDynamicMaterialInstance` _containerdoorr 0 (`PrimitiveComponent.GetMaterial` _containerdoorr 0)))
  (`MaterialInstanceDynamic.SetVectorParameterValue` _returnvalue_3 "diffuse color" (`self.ContainerColor`)))